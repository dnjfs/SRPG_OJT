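; BP_HitText is a short-lived floating text actor, named for hit feedback, that animates a text render component and then removes itself.
; On BeginPlay it stores its start location, and a timeline offsets the text's world position along Z from there, destroying the actor when finished.
; The construction script is empty; nodes for red, centered, resized text exist but are disconnected, and nothing here sets the displayed text.
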(event EventBeginPlay
  (Variables|Default|SetStartPos (Transformation|GetActorLocation))
  (bind _새_트랙_0 (Timeline|HitTextTimeLine Play)
    (:Update
      (Transformation|SetWorldLocation (Variables|Default|GetTextRender) (+ (Variables|Default|GetStartPos) (Math|Vector|MakeVector 0.0 0.0 (.Z (Math|Vector|BreakVector _새_트랙_0)))) false false))
    (:Finished
      (Actor|DestroyActor))))

(event Collision|EventActorBeginOverlap
  (params (OtherActor :type Actor%20Object%20Reference)))

(event EventTick
  (params (DeltaSeconds :type Float%20%28single-precision%29)))

(fn ConstructionScript)